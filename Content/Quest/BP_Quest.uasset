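; BP_Quest is a quest Blueprint that tracks completion through a hierarchy of sub-tasks.
; CheckQuestProgression marks the quest finished only when every ToDoList entry is finished, then calls FinishQuest.
; FinishQuest sets IsFinished and has a valid Referent recheck its own progression, so completion bubbles upward.
; Only a quest without a valid Referent fires the OnQuestFinished dispatcher.
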(fn `CheckQuestProgression`
  (set `self.IsFinished` true)
  (for _index (range (`KismetArrayLibrary.Array_Length` (`self.ToDoList`)))
    (if (not (`/Game/Quest/BP_Quest.IsFinished` (`|GetArrayItem` (`self.ToDoList`) _index)))
      (set `self.IsFinished` false)
      (break)))
  (if (`self.IsFinished`)
    (`self.FinishQuest`)))

(fn `FinishQuest`
  (bind _referent (`self.Referent`))
  (set `self.IsFinished` true)
  (`/Engine/EditorBlueprintResources/StandardMacros.IsValid` _referent
    (:`Is Valid`
      (`self.CheckQuestProgression` _referent))
    (:`Is Not Valid`
      (`self.OnQuestFinished`))))

(fn `UserConstructionScript`)