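; Quest puzzle generator that checks whether batteries in its green, red and blue slots match the solution colours.
; BeginPlay registers the slots and tints the cube's dynamic material cyan.
; CheckGenerator compares every slot through CompareColor, then fires the solved event and finishes the associated quest, or fires the failed event.
; CheckEmplacement validates a given slot, but its loop returns on the first iteration.
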(event `self.ReceiveBeginPlay`
  (bind _emplacements (`self.Emplacements`))
  (`self.ChangementCouleur`)
  (`KismetArrayLibrary.Array_Add` _emplacements (`self.BPC_Vert`))
  (`KismetArrayLibrary.Array_Add` _emplacements (`self.BPC_Rouge`))
  (`KismetArrayLibrary.Array_Add` _emplacements (`self.BPC_Bleu`)))

(fn `ChangementCouleur`
  (`MaterialInstanceDynamic.SetVectorParameterValue` (`self.MaterialInstance`) "Couleur" (struct :`G` 0.962675 :`B` 1.0 :`A` 1.0)))

(fn `CheckEmplacement`
  (params (EmplacementAVerif :type "/Game/Quest/BPC_Emplacement Object Reference"))
  (returns (Good :type Boolean))
  (locals (int :type Integer) (GoodOrNot :type Boolean))
  (set `local.int` 0)
  (for _index (range (`KismetArrayLibrary.Array_Length` (`self.Emplacements`)))
    (if (== EmplacementAVerif (`|GetArrayItem` (`self.Emplacements`) _index))
      (bind _same (`self.CompareColor` _index))
      (if _same
        (set `local.GoodOrNot` true)
        (else
          (set `local.GoodOrNot` false :!label _label)))
      (else
        (goto _label)))
    (return (`local.GoodOrNot`))))

(fn `CheckGenerator`
  (locals (Result :type Boolean))
  (set `local.Result` true)
  (for _index (range (`KismetArrayLibrary.Array_Length` (`self.Solutions`)))
    (bind _same (`self.CompareColor` _index))
    (if (not _same)
      (set `local.Result` false)
      (break)))
  (if (`local.Result`)
    (`self.EnigmeResolue`)
    (`/Game/Quest/BP_Quest.FinishQuest` (`self.AssociateQuest`))
    (else
      (`self.EnigmeRate`))))

(fn `CompareColor`
  (params (Int :type Integer))
  (returns (Same :type Boolean))
  (return (`|EnumEquality` (`|GetArrayItem` (`self.Solutions`) Int) (`/Game/Quest/BP_Batterie.Couleur` (`/Game/Quest/BPC_Emplacement.ActualBatterie` (`|GetArrayItem` (`self.Emplacements`) Int))))))

(fn `UserConstructionScript`
  (bind _returnvalue (`PrimitiveComponent.CreateDynamicMaterialInstance` (`self.Cube`) 0 "/Game/Quest/MI_Generateur.MI_Generateur" "None"))
  (set `self.MaterialInstance` _returnvalue))