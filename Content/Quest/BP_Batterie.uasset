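; BP_Batterie is a colored battery quest item that completes its associated quest when taken.
; The construction script creates a dynamic instance of MI_Batteries on the Cylinder, and BeginPlay tints it blue, red or green from the Couleur enum.
; On Take, it calls FinishQuest on AssociatedQuest and hides itself by moving far below the world instead of being destroyed.
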(event `self.ReceiveBeginPlay`
  (`self.ChangementCouleur`))

(event `/Game/Quest/BPI_Transportable.Take`
  (`/Game/Quest/BP_Quest.FinishQuest` (`self.AssociatedQuest`))
  (`self.K2_SetActorLocation` (0.0 0.0 -10000.0)))

(fn `ChangementCouleur`
  (switch `/Game/Quest/BPE_Colors` (`self.Couleur`)
    (:`NewEnumerator0`
      (`MaterialInstanceDynamic.SetVectorParameterValue` (`self.MaterialInstance`) "Couleur" (struct :`R` 0.021752 :`B` 1.0 :`A` 1.0)))
    (:`NewEnumerator1`
      (`MaterialInstanceDynamic.SetVectorParameterValue` (`self.MaterialInstance`) "Couleur" (struct :`R` 1.0 :`G` 0.048514 :`A` 1.0)))
    (:`NewEnumerator2`
      (`MaterialInstanceDynamic.SetVectorParameterValue` (`self.MaterialInstance`) "Couleur" (struct :`R` 0.007438 :`G` 1.0 :`A` 1.0)))))

(fn `UserConstructionScript`
  (bind _returnvalue (`PrimitiveComponent.CreateDynamicMaterialInstance` (`self.Cylinder`) 0 "/Game/Quest/MI_Batteries.MI_Batteries" "None"))
  (set `self.MaterialInstance` _returnvalue))